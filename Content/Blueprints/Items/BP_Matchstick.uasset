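; BP_Matchstick is a usable item that creates a short-lived, flickering light.
; UseItem runs the parent logic, then spawns a fresh BP_Matchstick and calls FlickerLight on it.
; FlickerLight makes the Sphere block a custom trace channel, then after a random short delay plays a timeline driving PointLight intensity.
; Once LightDuration elapses, the sphere ignores that channel again and the actor destroys itself.
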(event `FlickerLight`
  (`PrimitiveComponent.SetCollisionResponseToChannel` (`self.Sphere`) "ECC_GameTraceChannel1" "ECR_Block")
  (`KismetSystemLibrary.Delay` (`KismetMathLibrary.RandomFloatInRange` 0.0 0.2))
  (bind (_direction _intensity) (`Timeline|Timeline_0`)
    (:`Update`
      (`LightComponent.SetIntensity` (`self.PointLight`) (* _intensity 5000.0))
      (`KismetSystemLibrary.Delay` (`self.LightDuration`))
      (`PrimitiveComponent.SetCollisionResponseToChannel` (`self.Sphere`) "ECC_GameTraceChannel1" "ECR_Ignore")
      (`self.K2_DestroyActor`))))

(fn `UseItem`
  (returns (bSuccess :type Boolean))
  (bind _bsuccess (`parent.UseItem`))
  (bind _returnvalue (`|SpawnActorFromClass` "BP_Matchstick_C" (`KismetMathLibrary.MakeTransform` (0.0 0.0 0.0)) "Undefined" "OverrideRootScale" null null))
  (`self.FlickerLight` _returnvalue)
  (return _bsuccess))

(fn `UserConstructionScript`
  (`parent.UserConstructionScript`))