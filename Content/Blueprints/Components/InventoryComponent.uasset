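; Inventory component that stores item slots in an array and toggles an inventory window widget, still partly built.
; ToggleInventory centers the window's anchors on the HUD canvas; LoadPersistInventory holds a similar toggle with sounds instead of loading.
; AddToStack caps at max stack size and passes overflow to AddToInventory, which only searches for partial stacks via HasPartialStack.
; Preparation, stack creation, query and saving functions are empty stubs.
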(fn `AddToInventory`
  (params (ContentToAdd :type "/Game/Blueprints/Framework/Structs/ST_Slot Structure"))
  (returns (bSuccess :type Boolean))
  (if (`.Stackable_25_51868F9D44948B9B6E27F6A5020B2CEB` (break `/Game/Blueprints/Framework/Structs/ST_Item` (break `/Game/Blueprints/Framework/Structs/ST_Slot` ContentToAdd)))
    (`self.HasPartialStack` (`local.ContentToAdd`))))

(fn `AddToStack`
  (params (SlotStructure :type "/Game/Blueprints/Framework/Structs/ST_Slot Structure") (SlotIndex :type Integer))
  (returns (bSuccess :type Boolean))
  (locals (CurrentStackQuantity :type Integer))
  (bind _slotstructure_itemstructure (break `/Game/Blueprints/Framework/Structs/ST_Slot` (`local.SlotStructure`)))
  (bind _slotindex (`local.SlotIndex`))
  (bind (_slotstructure_itemstructure_2 _slotstructure_quantity) (break `/Game/Blueprints/Framework/Structs/ST_Slot` (`local.SlotStructure`)))
  (bind _inventory (`self.Inventory`))
  (bind (_slotstructure_itemstructure_3 _slotstructure_quantity_2) (break `/Game/Blueprints/Framework/Structs/ST_Slot` (`local.SlotStructure`)))
  (bind (_name _description _inventoryicon _pickupicon _quantity _stackable _maxstacksize) (break `/Game/Blueprints/Framework/Structs/ST_Item` _slotstructure_itemstructure))
  (bind _output (`|GetArrayItem` (`self.Inventory`) SlotIndex))
  (bind (_output_itemstructure _output_quantity) (break `/Game/Blueprints/Framework/Structs/ST_Slot` (`|GetArrayItem` _inventory _slotindex)))
  (bind _output_get (set `local.CurrentStackQuantity` (`.Quantity_5_3303960C477E645C816FC3BFE639D3FF` (break `/Game/Blueprints/Framework/Structs/ST_Slot` _output))))
  (if (> (+ _output_get (`.Quantity_5_3303960C477E645C816FC3BFE639D3FF` (break `/Game/Blueprints/Framework/Structs/ST_Slot` SlotStructure))) (`.MaxStackSize_27_E3F7D6BF439EA0C59DDD818234F1C651` (break `/Game/Blueprints/Framework/Structs/ST_Item` (break `/Game/Blueprints/Framework/Structs/ST_Slot` _output))))
    (`KismetArrayLibrary.Array_Set` (`self.Inventory`) (`local.SlotIndex`) (make `/Game/Blueprints/Framework/Structs/ST_Slot` _slotstructure_itemstructure _maxstacksize))
    (`self.AddToInventory` (make `/Game/Blueprints/Framework/Structs/ST_Slot` _slotstructure_itemstructure_2 (- _slotstructure_quantity (- _maxstacksize (`local.CurrentStackQuantity`)))))
    (else
      (`KismetArrayLibrary.Array_Set` _inventory _slotindex (make `/Game/Blueprints/Framework/Structs/ST_Slot` _output_itemstructure (+ _output_quantity _slotstructure_quantity_2)))))
  (return true))

(fn `CreateStack`)

(fn `InventoryQuery`)

(fn `LoadPersistInventory`
  (`self.InventoryWindow`
    (:`then`
      (`GameplayStatics.PlaySound2D` null 1.0 1.0 0.0 null null)
      (`Widget.RemoveFromParent` (`self.InventoryWindow`))
      (set `self.InventoryWindow` null))
    (:`else`
      (`GameplayStatics.PlaySound2D` null 1.0 1.0 0.0 null null)
      (`self.PrepareInventory`)
      (bind _returnvalue (`|CreateWidget` "/Game/Widgets/InventoryComponent/WBP_InventoryWindow.WBP_InventoryWindow_C" null self))
      (set `self.InventoryWindow` _returnvalue)
      (cast `/Game/Blueprints/Player/BP_PlayerController` (`GameplayStatics.GetPlayerController` 0)))))

(fn `PrepareInventory`)

(fn `SavePersistInventory`)

(fn `ToggleInventory`
  (`self.InventoryWindow`
    (:`then`
      (`Widget.RemoveFromParent` (`self.InventoryWindow`))
      (set `self.InventoryWindow` null))
    (:`else`
      (`self.PrepareInventory`)
      (bind _returnvalue (`|CreateWidget` "/Game/Widgets/InventoryComponent/WBP_InventoryWindow.WBP_InventoryWindow_C" null self))
      (set `self.InventoryWindow` _returnvalue)
      (bind _asbp_hud (cast `/Game/Blueprints/Framework/BP_HUD` (`PlayerController.GetHUD` (`GameplayStatics.GetPlayerController` 0))))
      (bind _returnvalue_2 (`CanvasPanel.AddChildToCanvas` (`/Game/Blueprints/Framework/BP_HUD.HUDCanvas` _asbp_hud) (`self.InventoryWindow`)))
      (`CanvasPanelSlot.SetAutoSize` _returnvalue_2 true)
      (`CanvasPanelSlot.SetAlignment` _returnvalue_2 (0.5 0.5))
      (`CanvasPanelSlot.SetAnchors` _returnvalue_2 (make `Anchors` (0.5 0.5) (0.5 0.5)))
      (`CanvasPanelSlot.SetPosition` _returnvalue_2 (`self.Position`)))))